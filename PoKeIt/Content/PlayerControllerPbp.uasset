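; Player controller Blueprint for a poker game that relays community card events to the HUD widget.
; SetHudWidget stores the widget reference, and SpawnCommunityCardsBP branches on the round stage to spawn the flop, turn or river on it.
; UpdateHUDcardsBP and DebugBlueprintFunc only print debug messages, as the hand update call on the widget is left unconnected.
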(event EventBeginPlay)

(event EventTick
  (params (DeltaSeconds :type Float%20%28single-precision%29)))

(event EventDebugBlueprintFunc
  (Development|PrintString "debugBlueprintFunc was called!" true true "(R=0.675000,G=0.000000,B=0.665248,A=1.000000)"))

(event EventUpdateHUDcardsBP
  (Development|PrintString "event updateHUDcards was called!" true true "(R=0.675000,G=0.000000,B=0.665248,A=1.000000)"))

(event EventSpawnCommunityCardsBP
  (params (roundStage :type Integer))
  (bind _hudwidget (Variables|Default|GethudWidget))
  (Development|PrintString "eventSpawnCopmmunityCardsBP was called!" true true "(R=0.675000,G=0.000000,B=0.665248,A=1.000000)")
  (if (== roundStage 0)
    (Default|SpawnFlop _hudwidget)
    (elif (== roundStage 1)
      (Default|SpawnTurn _hudwidget)
      (elif (== roundStage 2)
        (Default|SpawnRiver _hudwidget)))))

(fn ConstructionScript)

(fn SetHudWidget
  (params (hw :type HU%20Dwidget%20Object%20Reference))
  (Variables|Default|SethudWidget hw))