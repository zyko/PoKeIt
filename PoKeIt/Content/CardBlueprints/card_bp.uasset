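; Playing card actor that flips over and back and shows a face picture chosen by color and value.
; Rotate and Unrotate share the CardRotate timeline, played forward or in reverse to lerp position and pitch, with a sound and flip effect.
; Two gates re-arm each other so the flips alternate.
; SetCardPicture offsets a dynamic material's Translation parameter to select the picture, a method marked as temporary.
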(event Custom|Rotate
  (bind _returnvalue (Transformation|GetActorRotation))
  (bind (_roll _pitch _yaw) (Math|Rotator|BreakRotator _returnvalue))
  (bind _returnvalue_2 (Math|Rotator|MakeRotator _roll 179.0 _yaw))
  (bind _returnvalue_3 (Math|Rotator|MakeRotator _roll 359.0 _yaw))
  ;[1 1 1] Rotate Card
  (Utilities|FlowControl|Sequence
    (:then_0
      (Utilities|FlowControl|Gate false :!label _label
        (:Exit
          (Utilities|FlowControl|Sequence
            (:then_0
              (Variables|Default|SetStartPosition (Transformation|GetActorLocation))
              (Variables|Default|SetTempPosition (+ (Variables|Default|GetStartPosition) "0,0.000000,50.000000"))
              (Variables|Default|SetStartRotation _returnvalue_3)
              (Variables|Default|SetEndRotation _returnvalue_2)
              ;;[1 1 1] Sound Cards Rotate
              (Utilities|FlowControl|Sequence
                (:then_0
                  (Utilities|FlowControl|Delay 0.05)
                  (bind (_direction _angle _move) (Timeline|Card%20Rotate PlayFromStart)
                    (:Update
                      (Transformation|SetActorRelativeTransform (Math|Transform|MakeTransform (Math|Vector|Lerp(Vector) (Variables|Default|GetStartPosition) (Variables|Default|GetTempPosition) _move) (Math|Rotator|Lerp(Rotator) (Variables|Default|GetStartRotation) (Variables|Default|GetEndRotation) _angle) (Transformation|GetActorScale3D)) false false))))
                (:then_1
                  (Audio|PlaySoundatLocation 0 "0, 0, 0")
                  (Components|Activation|Activate (Variables|Components|GetFlip%20effect) false))))
            (:then_1
              (goto _label Close))))))
    (:then_1
      (Utilities|FlowControl|Gate true) ; enters at Open
    )))

(event Custom|Unrotate
  (bind _returnvalue (Transformation|GetActorRotation))
  (bind (_roll _pitch _yaw) (Math|Rotator|BreakRotator _returnvalue))
  (bind _returnvalue_2 (Math|Rotator|MakeRotator _roll 179.0 _yaw))
  (bind _returnvalue_3 (Math|Rotator|MakeRotator _roll 359.0 _yaw))
  ;[1 1 1] Rotate Card
  (Utilities|FlowControl|Sequence
    (:then_0
      (Utilities|FlowControl|Gate true :!label _label
        (:Exit
          (Utilities|FlowControl|Sequence
            (:then_0
              (Variables|Default|SetTempPosition (Transformation|GetActorLocation))
              (Variables|Default|SetStartPosition (Variables|Default|GetTempPosition))
              (Variables|Default|SetStartRotation _returnvalue_2)
              (Variables|Default|SetEndRotation _returnvalue_3)
              ;;[1 1 1] Sound Cards Rotate
              (Utilities|FlowControl|Sequence
                (:then_0
                  (Audio|PlaySoundatLocation 0 "0, 0, 0")
                  (Components|Activation|Activate (Variables|Components|GetFlip%20effect) false))
                (:then_1
                  (Utilities|FlowControl|Delay 0.05)
                  (bind (_direction _angle _move) (Timeline|Card%20Rotate ReverseFromEnd)
                    (:Update
                      (Transformation|SetActorRelativeTransform (Math|Transform|MakeTransform (Math|Vector|Lerp(Vector) (Variables|Default|GetStartPosition) (Variables|Default|GetTempPosition) _move) (Math|Rotator|Lerp(Rotator) (Variables|Default|GetStartRotation) (Variables|Default|GetEndRotation) _angle) (Transformation|GetActorScale3D)) false false))))))
            (:then_1
              (goto _label Close))))))
    (:then_1
      (Utilities|FlowControl|Gate false) ; enters at Open
    )))

(fn ConstructionScript)

(fn SetCardPicture
  (params (color :type Integer) (value :type Integer))
  (Variables|Default|Setcolor color)
  (Variables|Default|Setvalue value)
  (bind _returnvalue (Rendering|Material|CreateDynamicMaterialInstance (Variables|Default|GetCardPicture) 1 0 :!class /Script/Engine.PrimitiveComponent))
  (LocalVariables|SetMaterialDynamic _returnvalue)
  (Rendering|Material|SetVectorParameterValue (LocalVariables|GetMaterialDynamic) "Translation" (Math|Color|MakeColor (* (Math|Conversions|ToFloat(Integer) (Variables|Default|Getvalue)) 0.996) (Math|Conversions|ToFloat(Integer) (Variables|Default|Getcolor)) 0.0) :!class /Script/Engine.MaterialInstanceDynamic)
  (Rendering|Material|SetMaterial (Variables|Default|GetCardPicture) 1 (LocalVariables|GetMaterialDynamic)))